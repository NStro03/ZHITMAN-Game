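; Ribbon pickup actor that acts as the game's win trigger.
; Overlapping its box trigger sets the GotTheRibbon flag, plays a pickup sound, prints a message and destroys the actor.
; It then immediately runs the win moment: stops the first-person character's background sound, plays the win sound, shows the Win widget with the mouse cursor and pauses the game.
; The overlap does not filter which actor enters the trigger.
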(event `self.Ribbon_Box_Trigger.OnComponentBeginOverlap`
  (params (OverlappedComponent :type "PrimitiveComponent Object Reference") (OtherActor :type "Actor Object Reference") (OtherComp :type "PrimitiveComponent Object Reference") (OtherBodyIndex :type Integer) (bFromSweep :type Boolean) (SweepResult :type "HitResult Structure (by ref)"))
  ;[1 1 1] Ribbon pickup
  (set `self.Got_the_ribbon?` true)
  (`GameplayStatics.PlaySoundAtLocation` "/Game/GameAudio/Pickup.Pickup" (`SceneComponent.K2_GetComponentLocation` (`self.Ribbon`)) (struct) 1.0 1.0 0.0 null null null)
  (`KismetSystemLibrary.PrintString` "Ribbon Picked Up!")
  (`self.K2_DestroyActor`)
  ;[1 1 1] Win Moment
  (if (`self.Got_the_ribbon?`)
    (bind _asfirst_person_character (cast `/Game/FirstPersonBP/Blueprints/FirstPersonCharacter` (`GameplayStatics.GetPlayerCharacter` 0)))
    (`AudioComponent.Stop` (`/Game/FirstPersonBP/Blueprints/FirstPersonCharacter.Background Sound` _asfirst_person_character))
    (`GameplayStatics.PlaySound2D` "/Game/Shradha/Audios/win_sound.win_sound" 1.0 1.0 0.0 null null)
    (bind _returnvalue (`|CreateWidget` "/Game/Shradha/Interface_Widgets/Win_Widget.Win_Widget_C"))
    (`UserWidget.AddToViewport` _returnvalue 0)
    (set `PlayerController.bShowMouseCursor` true (`GameplayStatics.GetPlayerController` 0))
    (`GameplayStatics.SetGamePaused` true)))

(fn `UserConstructionScript`)