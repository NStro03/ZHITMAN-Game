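; Donut pickup actor that spins around its yaw axis at RotPerSecond and is collected on overlap with its DonutArea.
; BeginPlay caches the player's FirstPersonCharacter.
; Any overlap, with no check on the other actor, applies negative damage to that player, presumably as healing, and calls its PickupDiamond.
; It then plays an eating sound, spawns a collectable particle effect and destroys itself.
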(event `self.ReceiveBeginPlay`
  ;[1 1 1] DonutPickup1
  (bind _asfirst_person_character (cast `/Game/FirstPersonBP/Blueprints/FirstPersonCharacter` (`GameplayStatics.GetPlayerCharacter` 0)))
  (set `self.Player` _asfirst_person_character))

(event `self.DonutArea.OnComponentBeginOverlap`
  (params (OverlappedComponent :type "PrimitiveComponent Object Reference") (OtherActor :type "Actor Object Reference") (OtherComp :type "PrimitiveComponent Object Reference") (OtherBodyIndex :type Integer) (bFromSweep :type Boolean) (SweepResult :type "HitResult Structure (by ref)"))
  (bind _returnvalue (`self.K2_GetActorLocation`))
  (bind _player (`self.Player`))
  ;[1 1 1] DonutPickup
  (`|ExecutionSequence`
    (:`then_0`
      (`GameplayStatics.ApplyDamage` _player -2.0))
    (:`then_1`
      (`/Game/FirstPersonBP/Blueprints/FirstPersonCharacter.Pickup_Diamond` _player)
      (`GameplayStatics.PlaySoundAtLocation` "/Game/GameAudio/Eat_1.Eat_1" _returnvalue (struct) 1.0 1.0 0.0 null null null)
      (`GameplayStatics.SpawnEmitterAtLocation` "/Game/Cute_Zombie_Killing/Particles/p_collectable.p_collectable" _returnvalue)
      (`self.K2_DestroyActor`))))

(event `self.ReceiveTick`
  (params (DeltaSeconds :type "Float (single-precision)"))
  ;[1 1 1] Roation
  (`self.K2_AddActorWorldRotation` (`KismetMathLibrary.MakeRotator` 0.0 0.0 (* DeltaSeconds (`self.RotPerSecond`)))))

(fn `UserConstructionScript`)