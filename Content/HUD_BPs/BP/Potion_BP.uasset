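; Potion_BP is a health potion pickup that spins in the world and heals whatever actor overlaps it.
; Overlapping HealthTrigger applies negative damage to heal, plays the potion sound, spawns a particle emitter and destroys the actor.
; A delayed emitter cleanup follows the destroy call in the same chain.
; Tick adds yaw rotation scaled by delta time and RotPerSecond.
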(event `self.HealthTrigger.OnComponentBeginOverlap`
  (params (OverlappedComponent :type "PrimitiveComponent Object Reference") (OtherActor :type "Actor Object Reference") (OtherComp :type "PrimitiveComponent Object Reference") (OtherBodyIndex :type Integer) (bFromSweep :type Boolean) (SweepResult :type "HitResult Structure (by ref)"))
  (bind _returnvalue (`self.K2_GetActorLocation`))
  ;[1 1 1] PotionCollection
  (`GameplayStatics.ApplyDamage` OtherActor -25.0)
  (`GameplayStatics.PlaySoundAtLocation` "/Game/GameAudio/potion.potion" _returnvalue (struct) 1.0 1.0 0.0 null null null)
  (bind _returnvalue_2 (`GameplayStatics.SpawnEmitterAtLocation` null _returnvalue))
  (`self.K2_DestroyActor`)
  (`KismetSystemLibrary.Delay` 2.0)
  (`ActorComponent.K2_DestroyComponent` _returnvalue_2))

(event `self.ReceiveTick`
  (params (DeltaSeconds :type "Float (single-precision)"))
  ;[1 1 1] Rotation
  (`self.K2_AddActorWorldRotation` (`KismetMathLibrary.MakeRotator` 0.0 0.0 (* DeltaSeconds (`self.RotPerSecond`)))))

(fn `UserConstructionScript`)