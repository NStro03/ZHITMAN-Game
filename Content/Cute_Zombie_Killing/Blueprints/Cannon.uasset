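; Automatic cannon turret that tracks the FirstPersonCharacter and fires projectiles at it.
; Tick aims within range, yawing Platform and pitching CannonRotator at constant speed in actor-local space, otherwise easing both back to rest.
; An alignment check against TargetAimRotator, whose only assignment is unwired, starts firing through a DoOnce or stops it.
; The TurretRefire timeline serves as the refire timer, spawning a projectile each cycle while CanShoot holds.
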(event `self.ReceiveBeginPlay`
  ;[1 1 1] Get Target
  (bind _outactors (`GameplayStatics.GetAllActorsOfClass` "/Game/FirstPersonBP/Blueprints/FirstPersonCharacter.FirstPersonCharacter_C"))
  (set `self.Target` (`|GetArrayItem` _outactors)))

(event `ContinueFiring`
  ;[1 1 1] Fire At Target
  (if (`self.CanShoot`)
    (if (== (`TimelineComponent.GetPlaybackPosition` (`self.TurretRefire`)) 0.0) :!label _label
      (`self.FireProjectile`)
      (`Timeline|TurretRefire` :!label _label_2
        (:`Finished`
          (`self.ResetFireTimeline`)
          (`self.ContinueFiring`))))))

(event `StartFiring`
  ;[1 1 1] Fire At Target
  (`TimelineComponent.SetTimelineLength` (`self.TurretRefire`) (`self.RefireDelay`))
  (goto _label))

(event `ResetFireTimeline`
  ;[1 1 1] Fire At Target
  (`|ExecutionSequence`
    (:`then_0`
      (goto _label_2 :!via `Stop`))
    (:`then_1`
      (goto _label_2 :!via `SetNewTime`))))

(event `self.ReceiveTick`
  (params (DeltaSeconds :type "Float (single-precision)"))
  ;[1 1 1] Get Target Location
  (set `self.TargetLocation` (`self.K2_GetActorLocation` (`self.Target`)))
  ;[1 1 1] Check Target Distance
  (if (<= (`KismetMathLibrary.VSize` (- (`self.K2_GetActorLocation`) (`self.TargetLocation`))) 1024.0)
    (`self.AimAtTarget`)
    (else
      (`self.ResetAim`))))

(event `StopFiring`
  ;[1 1 1] Fire At Target
  (set `self.CanShoot` false)
  (`self.ResetFireTrigger`))

(event `FireProjectile`
  ;[1 1 1] Fire At Target
  (`/Engine/EditorBlueprintResources/StandardMacros.IsValid` (`self.Target`)
    (:`Is Valid`
      (`|SpawnActorFromClass` "/Game/Cute_Zombie_Killing/Blueprints/Projectile.Projectile_C" (`KismetMathLibrary.MakeTransform` (.location (`SceneComponent.K2_GetComponentToWorld` (`self.Cannon_Rotator`))) (.rotation (`SceneComponent.K2_GetComponentToWorld` (`self.Cannon_Rotator`)))) "Undefined" "OverrideRootScale" null null))
    (:`Is Not Valid`
      (`self.StopFiring`))))

(event `ResetAim`
  ;[1 1 1] Reset Aim
  (`SceneComponent.K2_SetRelativeRotation` (`self.Platform`) (`KismetMathLibrary.RInterpTo_Constant` (`SceneComponent.RelativeRotation` (`self.Platform`)) (struct) (`GameplayStatics.GetWorldDeltaSeconds`) 120.0) false false)
  (`SceneComponent.K2_SetRelativeRotation` (`self.Cannon_Rotator`) (`KismetMathLibrary.RInterpTo_Constant` (`SceneComponent.RelativeRotation` (`self.Cannon_Rotator`)) (struct) (`GameplayStatics.GetWorldDeltaSeconds`) 120.0) false false))

(event `AimAtTarget`
  (bind _returnvalue (`KismetMathLibrary.MakeRotFromX` (`KismetMathLibrary.InverseTransformDirection` (`self.GetTransform`) (- (`self.TargetLocation`) (`SceneComponent.K2_GetComponentLocation` (`self.Cannon_Rotator`))))))
  ;[1 1 1] Aim At Target
  (`SceneComponent.K2_SetRelativeRotation` (`self.Platform`) (`KismetMathLibrary.RInterpTo_Constant` (`SceneComponent.RelativeRotation` (`self.Platform`)) (`KismetMathLibrary.MakeRotator` 0.0 0.0 (.yaw _returnvalue)) (`GameplayStatics.GetWorldDeltaSeconds`) 120.0) false false)
  (`SceneComponent.K2_SetRelativeRotation` (`self.Cannon_Rotator`) (`KismetMathLibrary.RInterpTo_Constant` (`SceneComponent.RelativeRotation` (`self.Cannon_Rotator`)) (`KismetMathLibrary.MakeRotator` 0.0 (.pitch _returnvalue)) (`GameplayStatics.GetWorldDeltaSeconds`) 120.0) false false)
  (if (== (`self.TargetAimRotator`) (`KismetMathLibrary.MakeRotator` 0.0 (.pitch (`SceneComponent.RelativeRotation` (`self.Cannon_Rotator`))) (.yaw (`SceneComponent.RelativeRotation` (`self.Platform`)))) :`ErrorTolerance` 1.0)
    (`|ExecutionSequence`
      (:`then_0`
        (`/Engine/EditorBlueprintResources/StandardMacros.DoOnce` false :!label _label_3
          (:`Completed`
            (set `self.CanShoot` true)
            (`self.StartFiring`)))))
    (else
      (`self.StopFiring`))))

(event `ResetFireTrigger`
  ;[1 1 1] Aim At Target
  (goto _label_3 :!via `Reset`))

(fn `UserConstructionScript`)