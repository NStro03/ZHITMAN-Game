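; Fire hazard actor that deals environmental damage over time once an actor overlaps it.
; BeginPlay caches the player pawn as a FirstPersonCharacter.
; On overlap, a Delay-based loop applies damage to the overlapping actor every second while the cached player's Health is at least zero.
; The loop has no end-overlap exit, so leaving the fire does not stop it.
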(event `self.ReceiveBeginPlay`
  ;[1 1 1] Initialize Player
  (bind _asfirst_person_character (cast `/Game/FirstPersonBP/Blueprints/FirstPersonCharacter` (`GameplayStatics.GetPlayerPawn` 0)))
  (set `self.Player` _asfirst_person_character))

(event `self.ReceiveActorBeginOverlap`
  (params (OtherActor :type "Actor Object Reference"))
  ;[1 1 1] Damage on falling in Fire
  ;;[1 1 1] Workaround for Loop with Delay
  (if (>= (`/Game/FirstPersonBP/Blueprints/FirstPersonCharacter.Health` (`self.Player`)) 0.0) :!label _label
    (`|ExecutionSequence`
      (:`then_0`
        (`GameplayStatics.ApplyDamage` OtherActor 50.0 null null "/Engine/EngineDamageTypes/DmgTypeBP_Environmental.DmgTypeBP_Environmental_C"))
      (:`then_1`
        (`KismetSystemLibrary.Delay` 1.0)
        (goto _label)))))

(fn `UserConstructionScript`)