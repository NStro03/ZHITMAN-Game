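; Interactive Level 1 door: a first-person character inside the interaction box presses Interact to open or close it.
; Overlapping the box enables input and opens a gate; leaving disables both.
; Each press plays a button-push timeline, then a FlipFlop plays or reverses the door timeline, lerping the wall's Z between closed and open values.
; The construction script positions the button from a configurable transform.
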(event `InputAction|Interact`
  (params (Key :type "Key Structure"))
  (:`Pressed`
    (`/Engine/EditorBlueprintResources/StandardMacros.Gate` true :!label _label
      (:`Exit`
        (bind (_direction _button_track) (`Timeline|Button Press`)
          (:`Update`
            (`SceneComponent.K2_SetRelativeLocation` (`self.Button`) (`KismetMathLibrary.VLerp` (`self.Button Out`) (`self.Button In`) _button_track) false false))
          (:`Finished`
            (`/Engine/EditorBlueprintResources/StandardMacros.FlipFlop`
              (:`A`
                (bind (_direction_2 _door_track) (`Timeline|Door Timeline` :!label _label_2)
                  (:`Update`
                    (`SceneComponent.K2_SetRelativeLocation` (`self.Wall`) (`KismetMathLibrary.MakeVector` 0.0 0.0 (`KismetMathLibrary.Lerp` (`self.Door Close Value`) (`self.Door Open Value`) _door_track)) false false))))
              (:`B`
                (goto _label_2 :!via `Reverse`)))))))))

(event `self.Interaction Box.OnComponentBeginOverlap`
  (params (OverlappedComponent :type "PrimitiveComponent Object Reference") (OtherActor :type "Actor Object Reference") (OtherComp :type "PrimitiveComponent Object Reference") (OtherBodyIndex :type Integer) (bFromSweep :type Boolean) (SweepResult :type "HitResult Structure (by ref)"))
  (cast `/Game/FirstPersonBP/Blueprints/FirstPersonCharacter` OtherActor)
  (`self.EnableInput` (`GameplayStatics.GetPlayerController` 0))
  (goto _label :!via `Open`))

(event `self.Interaction Box.OnComponentEndOverlap`
  (params (OverlappedComponent :type "PrimitiveComponent Object Reference") (OtherActor :type "Actor Object Reference") (OtherComp :type "PrimitiveComponent Object Reference") (OtherBodyIndex :type Integer))
  (cast `/Game/FirstPersonBP/Blueprints/FirstPersonCharacter` OtherActor)
  (`self.DisableInput` (`GameplayStatics.GetPlayerController` 0))
  (goto _label :!via `Close`))

(fn `UserConstructionScript`
  (`SceneComponent.K2_SetRelativeTransform` (`self.Button`) (`self.Button Transform`) false false))