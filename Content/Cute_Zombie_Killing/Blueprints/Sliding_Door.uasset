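; Sliding door actor with two panels that opens when something overlaps PlayerTrigger and closes when the overlap ends.
; Separate timelines drive the relative Z of LowerDoor and UpperDoor, playing on begin overlap and reversing on end overlap, with no filter on the overlapping actor.
; Each timeline's update fires its open or close sound at world origin through a never-reset DoOnce, so each sound plays only once.
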(event `self.PlayerTrigger.OnComponentBeginOverlap`
  (params (OverlappedComponent :type "PrimitiveComponent Object Reference") (OtherActor :type "Actor Object Reference") (OtherComp :type "PrimitiveComponent Object Reference") (OtherBodyIndex :type Integer) (bFromSweep :type Boolean) (SweepResult :type "HitResult Structure (by ref)"))
  (`|ExecutionSequence`
    (:`then_0`
      (bind (_direction _newtrack_0) (`Timeline|slide_lower_door` :!label _label)
        (:`Update`
          (`SceneComponent.K2_SetRelativeLocation` (`self.lower_door`) (`KismetMathLibrary.MakeVector` 0.0 0.0 _newtrack_0) false false)
          (`/Engine/EditorBlueprintResources/StandardMacros.DoOnce` false
            (:`Completed`
              (`GameplayStatics.SpawnSoundAtLocation` "/Game/Shradha/Audios/doorOpen_002.doorOpen_002" (0.0 0.0 0.0) (struct) 1.0 1.0 0.0 null null))))))
    (:`then_1`
      (bind (_direction_2 _newtrack_0_2) (`Timeline|slide_upper_door` :!label _label_2)
        (:`Update`
          (`SceneComponent.K2_SetRelativeLocation` (`self.upper_door`) (`KismetMathLibrary.MakeVector` 0.0 0.0 _newtrack_0_2) false false)
          (`/Engine/EditorBlueprintResources/StandardMacros.DoOnce` false
            (:`Completed`
              (`GameplayStatics.SpawnSoundAtLocation` "/Game/Shradha/Audios/doorClose_002.doorClose_002" (0.0 0.0 0.0) (struct) 1.0 1.0 0.0 null null))))))))

(event `self.PlayerTrigger.OnComponentEndOverlap`
  (params (OverlappedComponent :type "PrimitiveComponent Object Reference") (OtherActor :type "Actor Object Reference") (OtherComp :type "PrimitiveComponent Object Reference") (OtherBodyIndex :type Integer))
  (`|ExecutionSequence`
    (:`then_0`
      (goto _label :!via `Reverse`))
    (:`then_1`
      (goto _label_2 :!via `Reverse`))))

(fn `UserConstructionScript`)